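; Player character for a 2D side-scroller, built on Paper2D flipbooks and Enhanced Input.
; Input drives X-axis movement with sprite flipping, jumping and level restart, and a quick double-tap of move switches from walking to running.
; Tick picks the idle, walk, run or jump flipbook from movement state, and returns the character to its start location when it falls below a height limit.
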(event Input|EnhancedActionEvents|EnhancedInputActionIA_Restart
  (params (ActionValue :type Boolean) (ElapsedSeconds :type Float%20%28double-precision%29) (TriggeredSeconds :type Float%20%28double-precision%29) (InputAction :type Input%20Action%20Object%20Reference :default "/Game/Input/Inputs/IA_Restart.IA_Restart"))
  (Game|OpenLevel(byName) "676767"))

(event Input|EnhancedActionEvents|EnhancedInputActionIA_Move
  (params (ActionValue :type Float%20%28double-precision%29) (ElapsedSeconds :type Float%20%28double-precision%29) (TriggeredSeconds :type Float%20%28double-precision%29) (InputAction :type Input%20Action%20Object%20Reference :default "/Game/Input/Inputs/IA_Move.IA_Move"))
  (bind _returnvalue (Utilities|Time|GetGameTimeinSeconds))
  (:Triggered
    (if (Variables|Default|GetCanMove)
      (Pawn|Input|AddMovementInput "1.000000,0.000000,0.000000" ActionValue false)
      (if (> ActionValue 0.0)
        (Transformation|SetRelativeRotation (Variables|Default|GetPaperFlipbook) "0, 0, 0" false false)
        (else
          (Transformation|SetRelativeRotation (Variables|Default|GetPaperFlipbook) "0.000000,180.000000,0.000000" false false)))
      (else
        (Development|PrintString "無法移動！"))))
  (:Started
    (if (<= (- _returnvalue (Variables|Default|GetLastTapTime)) 0.3)
      (Variables|Default|SetIsRunning true)
      (Variables|/Script/Engine.CharacterMovementComponent|SetMaxWalkSpeed (Variables|Character|GetCharacterMovement) 7e+02)
      (else
        (Variables|Default|SetIsRunning false)
        (Variables|/Script/Engine.CharacterMovementComponent|SetMaxWalkSpeed (Variables|Character|GetCharacterMovement) 3e+02)))
    (Variables|Default|SetLastTapTime _returnvalue)))

(event Input|EnhancedActionEvents|EnhancedInputActionIA_Jump
  (params (ActionValue :type Boolean) (ElapsedSeconds :type Float%20%28double-precision%29) (TriggeredSeconds :type Float%20%28double-precision%29) (InputAction :type Input%20Action%20Object%20Reference :default "/Game/Input/Inputs/IA_Jump.IA_Jump"))
  (:Started
    (Character|Jump)))

(event EventBeginPlay
  (Variables|Default|SetRespawnLocation (Transformation|GetActorLocation))
  (bind _returnvalue (Class|InputDeviceLibrary|GetPlayerControllerfromPlatformUser))
  (Input|AddMappingContext (PlayerController|LocalPlayerSubsystems|GetEnhancedInputLocalPlayerSubsystem _returnvalue) "/Game/Input/Inputs/IMC_Player.IMC_Player" 0 "(bIgnoreAllPressedKeysUntilRelease=True,bForceImmediately=False,bNotifyUserSettings=False)"))

(event Collision|EventActorBeginOverlap
  (params (OtherActor :type Actor%20Object%20Reference)))

(event EventTick
  (params (DeltaSeconds :type Float%20%28single-precision%29))
  (bind _paperflipbook (Variables|Default|GetPaperFlipbook))
  (if (< (.Z (Math|Vector|BreakVector (Transformation|GetActorLocation))) -3e+02)
    (Transformation|SetActorLocation (Variables|Default|GetRespawnLocation) false false)
    (Components|Movement|StopMovementImmediately (Variables|Character|GetCharacterMovement))
    (elif (AI|Components|NavMovement|IsFalling (Variables|Character|GetCharacterMovement))
      (Sprite|SetFlipbook (Variables|Default|GetPaperFlipbook) "/Game/Input/Flipbooks/FB_Jump.FB_Jump")
      (elif (> (Math|Vector|VectorLength (Transformation|GetVelocity)) 0.0)
        (if (Variables|Default|GetIsRunning)
          (Sprite|SetFlipbook _paperflipbook "/Game/Input/Flipbooks/FB_Run.FB_Run")
          (else
            (Sprite|SetFlipbook _paperflipbook "/Game/Input/Flipbooks/FB_Walk.FB_Walk")))
        (else
          (Sprite|SetFlipbook _paperflipbook "/Game/Input/Flipbooks/Idle.Idle"))))))

(fn ConstructionScript)