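; BP_Parallax is an actor that creates a horizontal parallax scrolling effect across three referenced background actors.
; On BeginPlay it caches the player character and the start locations of the player and the far, mid and near layers.
; Each Tick it offsets every layer from its start by a fraction of the player's X displacement, with the fraction increasing from far to near.
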(event EventBeginPlay
  (bind _output_get (Variables|Default|SetPlayerRef (Game|GetPlayerCharacter 0)))
  (Variables|Default|SetPlayerStartLocation (Transformation|GetActorLocation _output_get))
  (Variables|Default|SetBG_FarStartLocation (Transformation|GetActorLocation (Variables|Default|GetBG_FarRef)))
  (Variables|Default|SetBG_MidStartLocation (Transformation|GetActorLocation (Variables|Default|GetBG_MidRef)))
  (Variables|Default|SetBG_NearStartLocation (Transformation|GetActorLocation (Variables|Default|GetBG_NearRef))))

(event Collision|EventActorBeginOverlap
  (params (OtherActor :type Actor%20Object%20Reference)))

(event EventTick
  (params (DeltaSeconds :type Float%20%28single-precision%29))
  (bind _playerref (Variables|Default|GetPlayerRef))
  (bind _playerstartlocation (Variables|Default|GetPlayerStartLocation))
  (bind _returnvalue (Transformation|GetActorLocation _playerref))
  (bind _returnvalue_2 (- _returnvalue _playerstartlocation))
  (Transformation|SetActorLocation (Variables|Default|GetBG_FarRef) (+ (* _returnvalue_2 "0.100000,0.000000,0.000000") (Variables|Default|GetBG_FarStartLocation)) false false)
  (Transformation|SetActorLocation (Variables|Default|GetBG_MidRef) (+ (* _returnvalue_2 "0.150000,0.000000,0.000000") (Variables|Default|GetBG_MidStartLocation)) false false)
  (Transformation|SetActorLocation (Variables|Default|GetBG_NearRef) (+ (* _returnvalue_2 "0.200000,0.000000,0.000000") (Variables|Default|GetBG_NearStartLocation)) false false))

(fn ConstructionScript)